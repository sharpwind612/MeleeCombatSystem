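; Troll boss character that runs a behavior tree, carries a spawned sword and fights the player with melee and projectile attacks.
; First sight of the player creates the boss health bar and switches the blackboard behaviour enum.
; Attack events play montages and store their lengths, while a trace component receives the sword and enemy-tagged actors.
; Damage updates the bar; death stops AI, disables capsule collision and releases player lock-on.
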(event `self.ReceiveBeginPlay`
  ;[1 1 1] Set up enemy character
  (set `self.maxhealth` (`self.health`))
  (`AIController.RunBehaviorTree` (`AIBlueprintHelperLibrary.GetAIController` self) "/Game/Troll/Enemy/Enemy_Troll/BehaviourTree/Troll_BT.Troll_BT")
  (bind _returnvalue (`|SpawnActorFromClass` (`self.sword`) (`SceneComponent.GetSocketTransform` (`self.Mesh`) "sword" "RTS_World") "Undefined" "SelectDefaultAtRuntime" null null))
  (bind _output_get (set `self.swordref` _returnvalue))
  (`self.K2_AttachToComponent` _output_get (`self.Mesh`) "sword" "SnapToTarget" "SnapToTarget" "SnapToTarget" true)
  (set `/Game/Equipment/TraceComponent.swordref` (`self.swordref`) (`self.TraceComponent`))
  (bind _asbp_third_person_character (cast `/Game/ThirdPerson/Blueprints/BP_ThirdPersonCharacter` (`GameplayStatics.GetPlayerCharacter` 0)))
  (set `self.playerref` _asbp_third_person_character)
  (`BlackboardComponent.SetValueAsEnum` (`AIBlueprintHelperLibrary.GetBlackboard` null) "ebehaviour" (`self.behaviour`))
  (set `/Game/Equipment/RotatingComponent.Target` (`GameplayStatics.GetPlayerCharacter` 0) (`self.RotatingComponent`))
  (bind _outactors (`GameplayStatics.GetAllActorsWithTag` "enemy"))
  (set `/Game/Equipment/TraceComponent.enemy` _outactors (`self.TraceComponent`)))

(event `self.ReceiveAnyDamage`
  (params (Damage :type "Float (single-precision)") (DamageType :type "DamageType Object Reference") (InstigatedBy :type "Controller Object Reference") (DamageCauser :type "Actor Object Reference"))
  (bind _boss_healthbar (`self.boss healthbar`))
  (bind _playerref (`self.playerref`))
  ;[1 1 1] Damage system
  (bind _output_get (set `self.health` (- (`self.health`) Damage)))
  (`/Engine/EditorBlueprintResources/StandardMacros.IsValid` _boss_healthbar
    (:`Is Valid`
      (`/Game/Troll/Enemy/Enemy_Troll/Boss/BossHealthBar_WB.Updatehealthbar` _boss_healthbar)
      (if (<= _output_get 0.0)
        (`/Engine/EditorBlueprintResources/StandardMacros.DoOnce` false
          (:`Completed`
            (`BrainComponent.StopLogic` (`AIController.BrainComponent` (`AIBlueprintHelperLibrary.GetAIController` self)) "die")
            (`self.PlayAnimMontage` "/Game/Troll/Enemy/Enemy_Troll/Enemy_Troll_Poison_Animation/ExoGame_Troll_Death__Montage.ExoGame_Troll_Death__Montage")
            (`PrimitiveComponent.SetCollisionEnabled` (`self.CapsuleComponent`) "NoCollision")
            (`ActorComponent.K2_DestroyComponent` (`self.CharacterMovement`))
            (`Widget.RemoveFromParent` (`self.boss healthbar`))
            (if (== (`/Game/ThirdPerson/Blueprints/BP_ThirdPersonCharacter.TargetActor` _playerref) self)
              (`/Game/ThirdPerson/Blueprints/BP_ThirdPersonCharacter.DisengageLock` _playerref))))))))

(event `Attack`
  ;[1 1 1] Attack system
  (bind _returnvalue (`self.PlayAnimMontage` (`KismetArrayLibrary.Array_Random` (`self.attackanimations`))))
  (set `self.attacklength` _returnvalue))

(event `Projectileattack`
  ;[1 1 1] Play Projectile Attack Anim
  (bind _returnvalue (`self.PlayAnimMontage` "/Game/Troll/Enemy/Enemy_Troll/Enemy_Troll_Poison_Animation/ExoGame_Troll_Attack_Vomit_Montage.ExoGame_Troll_Attack_Vomit_Montage"))
  (set `self.rangedattacklength` _returnvalue))

(event `Fireprojectile`
  (bind _returnvalue (`SceneComponent.K2_GetComponentLocation` (`self.projetilespawnpoint`)))
  ;[1 1 1] Spawn Projectile Attack
  (`|SpawnActorFromClass` "/Game/Troll/Enemy/Enemy_Troll/Boss/BossProjectile_BP.BossProjectile_BP_C" (`KismetMathLibrary.MakeTransform` _returnvalue (`KismetMathLibrary.FindLookAtRotation` _returnvalue (`self.K2_GetActorLocation` (`GameplayStatics.GetPlayerCharacter` 0)))) "Undefined" "OverrideRootScale" null null))

(event `/Game/Lockon/LockononInterface.onselected`
  ;[1 1 1] Handle lock on
  (`SceneComponent.SetVisibility` (`self.Lockon`) true false))

(event `/Game/Lockon/LockononInterface.ondeselected`
  ;[1 1 1] Handle lock on
  (`SceneComponent.SetVisibility` (`self.Lockon`) false false))

(event `self.PawnSensing.OnSeePawn`
  (params (Pawn :type "Pawn Object Reference"))
  ;[1 1 1] Handle enemy vision
  (if (== Pawn (`GameplayStatics.GetPlayerCharacter` 0))
    (`/Engine/EditorBlueprintResources/StandardMacros.DoOnce` false
      (:`Completed`
        (bind _returnvalue (`|CreateWidget` "/Game/Troll/Enemy/Enemy_Troll/Boss/BossHealthBar_WB.BossHealthBar_WB_C" null self))
        (bind _output_get (set `self.boss healthbar` _returnvalue))
        (`UserWidget.AddToViewport` _output_get 0)
        (set `self.behaviour` "NewEnumerator3")
        (`BlackboardComponent.SetValueAsEnum` (`AIBlueprintHelperLibrary.GetBlackboard` null) "ebehaviour" (`self.behaviour`))))))

(event `Clear hit actors`
  ;[1 1 1] clear hit actors
  (`KismetArrayLibrary.Array_Clear` (`/Game/Equipment/TraceComponent.actorstoignore` (`self.TraceComponent`))))

(fn `isdead`
  (returns (`isdead?` :type Boolean))
  (return (`self.enemydead?`)))

(fn `UserConstructionScript`)