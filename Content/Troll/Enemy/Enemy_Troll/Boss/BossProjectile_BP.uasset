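; Boss projectile actor for the troll boss, which damages the third-person player character on contact.
; A sphere overlap with the player applies fixed damage, while a blocking hit on the actor deals none.
; Both events stop the projectile movement, swap the particle system to a thunder ball impact effect and destroy the actor after a short delay.
; Each event has its own DoOnce, so each fires only once.
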(event `self.Sphere.OnComponentBeginOverlap`
  (params (OverlappedComponent :type "PrimitiveComponent Object Reference") (OtherActor :type "Actor Object Reference") (OtherComp :type "PrimitiveComponent Object Reference") (OtherBodyIndex :type Integer) (bFromSweep :type Boolean) (SweepResult :type "HitResult Structure (by ref)"))
  (bind _asbp_third_person_character (cast `/Game/ThirdPerson/Blueprints/BP_ThirdPersonCharacter` OtherActor))
  (`/Engine/EditorBlueprintResources/StandardMacros.DoOnce` false
    (:`Completed`
      (`GameplayStatics.ApplyDamage` _asbp_third_person_character 10.0 null self)
      (`MovementComponent.StopMovementImmediately` (`self.ProjectileMovement`))
      (`ParticleSystemComponent.SetTemplate` (`self.ParticleSystem`) "/Game/MarketplaceAssets/FXVarietyPack/Particles/P_ky_ThunderBallHit.P_ky_ThunderBallHit")
      (`KismetSystemLibrary.Delay` 2.0)
      (`self.K2_DestroyActor`))))

(event `self.ReceiveHit`
  (params (MyComp :type "PrimitiveComponent Object Reference") (Other :type "Actor Object Reference") (OtherComp :type "PrimitiveComponent Object Reference") (bSelfMoved :type Boolean) (HitLocation :type "Vector Structure") (HitNormal :type "Vector Structure") (NormalImpulse :type "Vector Structure") (Hit :type "HitResult Structure (by ref)"))
  (`/Engine/EditorBlueprintResources/StandardMacros.DoOnce` false
    (:`Completed`
      (`MovementComponent.StopMovementImmediately` (`self.ProjectileMovement`))
      (`ParticleSystemComponent.SetTemplate` (`self.ParticleSystem`) "/Game/MarketplaceAssets/FXVarietyPack/Particles/P_ky_ThunderBallHit.P_ky_ThunderBallHit")
      (`KismetSystemLibrary.Delay` 2.0)
      (`self.K2_DestroyActor`))))

(fn `UserConstructionScript`)